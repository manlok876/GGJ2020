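; Elevator button actor that sends an elevator into action once the button has been activated.
; It starts with an inactive material on its Cylinder, and SetActive flags it active and swaps in the active material.
; Action does nothing while inactive; when active, it passes itself to TargetElevator's Action, or fires OnWinCondition if no valid elevator is set.
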(event `self.ReceiveBeginPlay`
  (bind _returnvalue (`PrimitiveComponent.CreateDynamicMaterialInstance` (`self.Cylinder`) 0 (`self.InactiveMaterial`) "None"))
  (set `self.MaterialInstance` _returnvalue))

(event `self.Action`
  (params (Instigator :type "Actor Object Reference"))
  (bind _targetelevator (`self.TargetElevator`))
  (if (`self.IsActive`)
    (`/Engine/EditorBlueprintResources/StandardMacros.IsValid` _targetelevator
      (:`Is Valid`
        (`/Game/Elevator/BP_Elevator.Action` _targetelevator self))
      (:`Is Not Valid`
        (`self.onWinCondition`)))))

(fn `SetActive`
  (set `self.IsActive` true)
  (`PrimitiveComponent.CreateDynamicMaterialInstance` (`self.Cylinder`) 0 (`self.ActiveMaterial`) "None"))

(fn `UserConstructionScript`)