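; Game mode for a GGJ2020 repair game that runs the HUD and decides win or loss.
; BeginPlay binds to player power, panel repairs and elevator win events, re-binding the buttons inside the panel loop.
; Each repair updates the HUD and counts down remaining panels, activating elevator buttons at zero.
; An elevator win or depleted power flags game over, pauses, and shows the matching widget with UI-only input.
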(event `onWinConditionGM`
  (bind _returnvalue (`GameplayStatics.GetPlayerController` 0))
  (bind _asbp_ggj2020game_state_base (cast `/Game/Game/BP_GGJ2020GameStateBase` (`GameplayStatics.GetGameState`)))
  (set `/Game/Game/BP_GGJ2020GameStateBase.IsGameOver` true _asbp_ggj2020game_state_base)
  (`GameplayStatics.SetGamePaused` true)
  (bind _returnvalue_2 (`|CreateWidget` "/Game/UI/WinWidget.WinWidget_C"))
  (bind _output_get (set `self.WinWidget` _returnvalue_2))
  (`UserWidget.AddToViewport` _output_get 0)
  (`WidgetBlueprintLibrary.SetInputMode_UIOnlyEx` _returnvalue null)
  (set `PlayerController.bShowMouseCursor` true _returnvalue))

(event `self.ReceiveBeginPlay`
  (bind _returnvalue (`GameplayStatics.GetPlayerController` 0))
  (bind _returnvalue_2 (`|CreateWidget` "/Game/UI/PlayerHUD.PlayerHUD_C" _returnvalue))
  (bind _output_get (set `self.PlayerHUD` _returnvalue_2))
  (`UserWidget.AddToPlayerScreen` _output_get 0)
  (`WidgetBlueprintLibrary.SetInputMode_GameOnly` _returnvalue)
  (bind _asggj2020character (cast `GGJ2020Character` (`GameplayStatics.GetPlayerCharacter` 0)))
  (bind _returnvalue_3 (`self.GetComponentByClass` _asggj2020character "/Script/GGJ2020.PowerActorComponent"))
  (set `self.PlayerPowerComponent` _returnvalue_3)
  (add `PowerActorComponent.OnPowerChanged` _returnvalue_3 (delegate `onPlayerPowerChanged`))
  (bind _outactors (`GameplayStatics.GetAllActorsOfClass` "/Game/Panels/Panel.Panel_C"))
  (set `self.PanelsToRepair` (`KismetArrayLibrary.Array_Length` _outactors))
  (for _array_element _outactors
    (add `/Game/Panels/Panel.OnRepairedDispatcher` _array_element (delegate `onPanelRepaired`))
    (bind _outactors_2 (`GameplayStatics.GetAllActorsOfClass` "/Game/Elevator/BP_ElevatorButton.BP_ElevatorButton_C"))
    (for _array_element_2 _outactors_2
      (add `/Game/Elevator/BP_ElevatorButton.onWinCondition` _array_element_2 (delegate `onWinConditionGM`)))))

(event `onPanelRepaired`
  (bind _panelstorepair (`self.PanelsToRepair`))
  (`/Game/UI/PlayerHUD.AddFixedPanel` (`self.PlayerHUD`))
  (`/Engine/EditorBlueprintResources/StandardMacros.DecrementInt` _panelstorepair
    (:`  `
      (if (<= _panelstorepair 0)
        (bind _outactors (`GameplayStatics.GetAllActorsOfClass` "/Game/Elevator/BP_ElevatorButton.BP_ElevatorButton_C"))
        (for _array_element _outactors
          (`/Game/Elevator/BP_ElevatorButton.SetActive` _array_element))))))

(event `onPlayerPowerChanged`
  (bind _returnvalue (`GameplayStatics.GetPlayerController` 0))
  (bind _aspower_actor_component (cast `PowerActorComponent` (`self.PlayerPowerComponent`)))
  (if (<= (`PowerActorComponent.GetPowerAmount` _aspower_actor_component) 0.0)
    (bind _asbp_ggj2020game_state_base (cast `/Game/Game/BP_GGJ2020GameStateBase` (`GameplayStatics.GetGameState`)))
    (set `/Game/Game/BP_GGJ2020GameStateBase.IsGameOver` true _asbp_ggj2020game_state_base)
    (`GameplayStatics.SetGamePaused` true)
    (bind _returnvalue_2 (`|CreateWidget` "/Game/UI/GameOverWidget.GameOverWidget_C"))
    (bind _output_get (set `self.GameOverWidget` _returnvalue_2))
    (`UserWidget.AddToViewport` _output_get 0)
    (`WidgetBlueprintLibrary.SetInputMode_UIOnlyEx` _returnvalue null)
    (set `PlayerController.bShowMouseCursor` true _returnvalue)))

(fn `UserConstructionScript`)